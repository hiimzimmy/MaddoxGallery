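; Actor Blueprint that reports its own length in metres as an on-screen debug message.
; On BeginPlay it takes the absolute Y difference between the relative locations of its two static mesh components and divides by 100 to convert to metres.
; It prints the result with the object's name in a long-lasting PrintString, and the construction script is empty.
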(event `self.ReceiveBeginPlay`
  (bind (_relativelocation_x _relativelocation_y) (`KismetMathLibrary.BreakVector` (`SceneComponent.RelativeLocation` (`self.StaticMesh1`))))
  (bind (_relativelocation_x_2 _relativelocation_y_2) (`KismetMathLibrary.BreakVector` (`SceneComponent.RelativeLocation` (`self.StaticMesh`))))
  (bind _output_get (set `self.Object Name` (`KismetSystemLibrary.GetObjectName` self)))
  (`KismetSystemLibrary.PrintString` (`KismetStringLibrary.Concat_StrStr` "The " _output_get " is " (`KismetStringLibrary.Conv_DoubleToString` (/ (`KismetMathLibrary.Abs` (- _relativelocation_y_2 _relativelocation_y)) 100.0)) " Metres long.") true true (struct :`G` 0.66 :`B` 1.0 :`A` 1.0) 2000.0))

(fn `UserConstructionScript`)